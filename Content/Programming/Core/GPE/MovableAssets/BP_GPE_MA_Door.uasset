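; Movable door gameplay element that opens or closes when its BPACOutput component fires, either once or repeatably.
; After a delay, a timeline scaled to the animation time plays or reverses to drive all attached BPAC_Animation components, while an optional smart camera with a fixed camera is triggered.
; The on/off state is saved through BPSG_Output and repositions animations on load.
; The construction script offsets the mesh by Height to preview the closed state.
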(event `self.ReceiveBeginPlay`
  (bind _bpac_output (`self.BPAC_Output`))
  ;[1 1 1] Initialisation - Bind
  (set `/Game/Programming/Core/GPE/MovableAssets/BPAC_Output.Action Repetable` (`self.Repetable`) _bpac_output)
  (set `/Game/Programming/Core/GPE/MovableAssets/BPAC_Output.Push Function` (`self.Push Function`) _bpac_output)
  (add `/Game/Programming/Core/GPE/MovableAssets/BPAC_Output.OnOutput` (`self.BPAC_Output`) (delegate `PillarMovement`))
  ;[1 1 1] Initialization of the timeline
  (`TimelineComponent.SetPlayRate` (`self.Timeline_0`) (/ 1.0 (`self.Time Animation`)))
  ;[1 1 1] Initialization for animation
  (for _array_element (`self.K2_GetComponentsByClass` "/Game/Programming/Core/GPE/MovableAssets/BPAC_Animation.BPAC_Animation_C")
    (bind _asbpac_animation (cast `/Game/Programming/Core/GPE/MovableAssets/BPAC_Animation` _array_element))
    (set `/Game/Programming/Core/GPE/MovableAssets/BPAC_Animation.Element` self _asbpac_animation)
    (`/Game/Programming/Core/GPE/MovableAssets/BPAC_Animation.Initialization` _asbpac_animation)))

(event `PillarMovement`
  ;[1 1 1] Door Movement
  (`self.ToggleDoor` (`self.On/Off`))
  (if (not (`self.Repetable`))
    (remove `/Game/Programming/Core/GPE/MovableAssets/BPAC_Output.OnOutput` (`self.BPAC_Output`) (delegate `PillarMovement`))))

(event `ToggleDoor`
  (params (Condition :type Boolean))
  (bind _returnvalue (`self.GetComponentByClass` "/Game/Programming/Core/DynamicCamera/BPAC_SmartCameraComponent.BPAC_SmartCameraComponent_C"))
  ;[1 1 1] Smooth Toggle
  (`|ExecutionSequence`
    (:`then_0`
      (`KismetSystemLibrary.Delay` (`self.Delay Before Action`))
      (if Condition
        (bind (_direction _newtrack_0) (`Timeline|Timeline_0` :!label _label)
          (:`Update`
            ;;[1 1 1] Animations
            (for _array_element (`self.K2_GetComponentsByClass` "/Game/Programming/Core/GPE/MovableAssets/BPAC_Animation.BPAC_Animation_C")
              (bind _asbpac_animation (cast `/Game/Programming/Core/GPE/MovableAssets/BPAC_Animation` _array_element))
              (`/Game/Programming/Core/GPE/MovableAssets/BPAC_Animation.Do Animation` _asbpac_animation _newtrack_0)))
          (:`Finished`
            (set `self.On/Off` (not Condition))))
        (else
          (goto _label :!via `Reverse`))))
    (:`then_1`
      ;;[1 1 1] Camera
      (`/Engine/EditorBlueprintResources/StandardMacros.IsValid` _returnvalue
        (:`Is Valid`
          (`/Engine/EditorBlueprintResources/StandardMacros.IsValid` (`/Game/Programming/Core/DynamicCamera/BPAC_SmartCameraComponent.Fixed Camera` _returnvalue)
            (:`Is Valid`
              (`/Game/Programming/Core/DynamicCamera/BPAC_SmartCameraComponent.ExternalTrigger` _returnvalue))))))))

(event `/Game/Programming/Core/Savers/BPI_Saveable.Load Data`
  (params (Data :type "SaveGame Object Reference"))
  ;[1 1 1 0.33] Load Save
  (bind _asbpsg_output (cast `/Game/Programming/Core/Savers/Data/BPSG_Output` Data))
  (bind _is_active (`/Game/Programming/Core/Savers/Data/BPSG_Output.Is Active` _asbpsg_output))
  ;;[1 1 1 0.33] Set Active on Change
  (if (!= _is_active (`self.On/Off`))
    (set `self.On/Off` _is_active)
    ;;[1 1 1 0.33] Repositioning
    (for _array_element (`self.K2_GetComponentsByClass` "/Game/Programming/Core/GPE/MovableAssets/BPAC_Animation.BPAC_Animation_C")
      (bind _asbpac_animation (cast `/Game/Programming/Core/GPE/MovableAssets/BPAC_Animation` _array_element))
      (`/Game/Programming/Core/GPE/MovableAssets/BPAC_Animation.Repositioning` _asbpac_animation (`self.On/Off`)))))

(fn `Get Save Data`
  (returns (Data :type "SaveGame Object Reference"))
  (bind _returnvalue (`GameplayStatics.CreateSaveGameObject` "/Game/Programming/Core/Savers/Data/BPSG_Output.BPSG_Output_C"))
  (set `/Game/Programming/Core/Savers/Data/BPSG_Output.Is Active` (`self.On/Off`) _returnvalue)
  (return _returnvalue))

(fn `UserConstructionScript`
  (bind _door (`self.Door`))
  ;[1 1 1] See the closed door in the editor
  (if (`self.Closed`)
    (`SceneComponent.K2_SetRelativeLocation` _door (+ (`SceneComponent.RelativeLocation` _door) (`KismetMathLibrary.MakeVector` 0.0 0.0 (`self.Height`))) false false)))