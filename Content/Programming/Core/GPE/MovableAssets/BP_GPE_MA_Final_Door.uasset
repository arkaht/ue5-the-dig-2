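; Final door puzzle asset that opens or closes when its BPACOutput component fires, once or repeatably.
; After a delay, a duration-scaled timeline drives BPAC_Animation on each attached part actor.
; Toggling also triggers an optional fixed smart camera and can spawn a configured actor at a socket after its own delay.
; A separate SpawnFinalDoor function spawns and attaches the four door parts unless a bottom part exists.
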(event `self.ReceiveBeginPlay`
  (bind _bpac_output (`self.BPAC_Output`))
  ;[1 1 1 0.33] Initialisation - Bind
  (set `/Game/Programming/Core/GPE/MovableAssets/BPAC_Output.Action Repetable` (`self.Repetable`) _bpac_output)
  (set `/Game/Programming/Core/GPE/MovableAssets/BPAC_Output.Push Function` (`self.Push Function`) _bpac_output)
  (add `/Game/Programming/Core/GPE/MovableAssets/BPAC_Output.OnOutput` (`self.BPAC_Output`) (delegate `PillarMovement`))
  ;[1 1 1 0.33] Initialization of the timeline
  (`TimelineComponent.SetPlayRate` (`self.Timeline_0`) (/ 1.0 (`self.Time Animation`))))

(event `PillarMovement`
  ;[1 1 1 0.33] Door Movement
  (`self.ToggleDoor` (`self.On/Off`))
  (if (not (`self.Repetable`))
    (remove `/Game/Programming/Core/GPE/MovableAssets/BPAC_Output.OnOutput` (`self.BPAC_Output`) (delegate `PillarMovement`))))

(event `ToggleDoor`
  (params (Condition :type Boolean))
  (bind _returnvalue (`self.GetComponentByClass` "/Game/Programming/Core/DynamicCamera/BPAC_SmartCameraComponent.BPAC_SmartCameraComponent_C"))
  (bind _spawn_actor_class_at_open (`self.Spawn Actor Class at Open`))
  ;[1 1 1 0.33] Smooth Toggle
  (`|ExecutionSequence`
    (:`then_0`
      (`KismetSystemLibrary.Delay` (`self.Delay Before Action`))
      (if Condition
        (bind (_direction _newtrack_0) (`Timeline|Timeline_0` :!label _label)
          (:`Update`
            ;;[1 1 1 0.33] Animations
            (for _array_element (`self.GetAttachedActors` true)
              (`/Game/Programming/Core/GPE/MovableAssets/BPAC_Animation.Do Animation` (`self.GetComponentByClass` _array_element "/Game/Programming/Core/GPE/MovableAssets/BPAC_Animation.BPAC_Animation_C") _newtrack_0)))
          (:`Finished`
            (set `self.On/Off` (not Condition))))
        (else
          (goto _label :!via `Reverse`))))
    (:`then_1`
      ;;[1 1 1 0.33] Camera
      (`/Engine/EditorBlueprintResources/StandardMacros.IsValid` _returnvalue
        (:`Is Valid`
          (`/Engine/EditorBlueprintResources/StandardMacros.IsValid` (`/Game/Programming/Core/DynamicCamera/BPAC_SmartCameraComponent.Fixed Camera` _returnvalue)
            (:`Is Valid`
              (`/Game/Programming/Core/DynamicCamera/BPAC_SmartCameraComponent.ExternalTrigger` _returnvalue))))))
    (:`then_2`
      ;;[1 1 1 0.33] Spawn Actor
      (if (`KismetSystemLibrary.IsValidClass` _spawn_actor_class_at_open)
        (`KismetSystemLibrary.Delay` (`self.Spawn Actor Delay`))
        (`|SpawnActorFromClass` _spawn_actor_class_at_open (`SceneComponent.K2_GetComponentToWorld` (`self.Spawn Actor Socket`)) "Undefined" "OverrideRootScale" null null)))))

(fn `Spawn Final Door`
  (locals (exist :type Boolean))
  (bind _returnvalue (`self.GetTransform`))
  (for _array_element (`self.GetAttachedActors` true)
    (cast `/Game/Programming/Core/GPE/MovableAssets/Parts/BP_GPE_MA_Final_Door_Bottom` _array_element)
    (set `local.exist` true))
  (if (not (`local.exist`))
    ;[1 1 1] Spawn all parts
    (bind _returnvalue_2 (`|SpawnActorFromClass` "/Game/Programming/Core/GPE/MovableAssets/Parts/BP_GPE_MA_Final_Door_Bottom.BP_GPE_MA_Final_Door_Bottom_C" _returnvalue "Undefined" "OverrideRootScale" null null))
    (`self.K2_AttachToActor` _returnvalue_2 self "None" "SnapToTarget" "SnapToTarget" "KeepRelative" true)
    (bind _returnvalue_3 (`|SpawnActorFromClass` "/Game/Programming/Core/GPE/MovableAssets/Parts/BP_GPE_MA_Final_Door_Left.BP_GPE_MA_Final_Door_Left_C" _returnvalue "Undefined" "OverrideRootScale" null null))
    (`self.K2_AttachToActor` _returnvalue_3 self "None" "SnapToTarget" "SnapToTarget" "KeepRelative" true)
    (bind _returnvalue_4 (`|SpawnActorFromClass` "/Game/Programming/Core/GPE/MovableAssets/Parts/BP_GPE_MA_Final_Door_Right.BP_GPE_MA_Final_Door_Right_C" _returnvalue "Undefined" "OverrideRootScale" null null))
    (`self.K2_AttachToActor` _returnvalue_4 self "None" "SnapToTarget" "SnapToTarget" "KeepRelative" true)
    (bind _returnvalue_5 (`|SpawnActorFromClass` "/Game/Programming/Core/GPE/MovableAssets/Parts/BP_GPE_MA_Final_Door_Top.BP_GPE_MA_Final_Door_Top_C" _returnvalue "Undefined" "OverrideRootScale" null null))
    (`self.K2_AttachToActor` _returnvalue_5 self "None" "SnapToTarget" "SnapToTarget" "KeepRelative" true)))

(fn `UserConstructionScript`)