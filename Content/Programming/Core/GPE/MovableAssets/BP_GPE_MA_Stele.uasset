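; BP_GPE_MA_Stele is a stele gameplay element whose material visually switches when its BPAC_Output component fires OnOutput.
; The construction script creates a dynamic material instance on the mesh with the "Switch" parameter at zero.
; The SwitchSettings timeline animates that parameter on each update.
; The FlipFlopDoOnce flag selects the behavior: true plays the timeline only once, false alternates playing and reversing it on each output.
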(event `self.BPAC_Output.OnOutput`
  (if (`self.FlipFlop / Do Once`)
    (`/Engine/EditorBlueprintResources/StandardMacros.DoOnce` false
      (:`Completed`
        (bind (_direction _newtrack_0) (`Timeline|SwitchSettings` :!label _label)
          (:`Update`
            (`MaterialInstanceDynamic.SetScalarParameterValue` (`self.Dynamic Stele Material`) "Switch" _newtrack_0)))))
    (else
      (`/Engine/EditorBlueprintResources/StandardMacros.FlipFlop`
        (:`A`
          (goto _label))
        (:`B`
          (goto _label :!via `Reverse`))))))

(fn `UserConstructionScript`
  (bind _returnvalue (`PrimitiveComponent.CreateDynamicMaterialInstance` (`self.Stele`) 0 "/Game/Art/3_MATERIALS/Instances/MAT_GPE_SteleDynamic.MAT_GPE_SteleDynamic" "None"))
  (bind _output_get (set `self.Dynamic Stele Material` _returnvalue))
  (`MaterialInstanceDynamic.SetScalarParameterValue` _output_get "Switch" 0.0))