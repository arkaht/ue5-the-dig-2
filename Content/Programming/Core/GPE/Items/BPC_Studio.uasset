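; BPC_Studio is an item inspection Blueprint that shows an inspection UI while the player's own input is suspended.
; Inspect stores the player, sets the ItemToFocus mesh with no mesh specified, adds a UI_Inspect widget to the viewport and moves input to itself.
; Pressing Interact hands input back to the player and removes the widget.
; The separate Interact function is a stub returning false.
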(event `/Game/Programming/Core/GPE/Items/Interface/I_Inspect.Inspect`
  (params (Player :type "/Game/Programming/Core/BPC_Player Object Reference") (ItemToFocus :type "StaticMeshComponent Object Reference") (ItemName :type Text) (ItemDescription :type Text))
  (bind _returnvalue (`GameplayStatics.GetPlayerController` 0))
  (set `self.Player` Player)
  (`StaticMeshComponent.SetStaticMesh` (`self.ItemToFocus`) null)
  (bind _returnvalue_2 (`|CreateWidget` "/Game/Programming/UI/UI_Inspect.UI_Inspect_C"))
  (bind _output_get (set `self.InspectionWidget` _returnvalue_2))
  (`UserWidget.AddToViewport` _output_get 0)
  (`self.DisableInput` (`self.Player`) _returnvalue)
  (`self.EnableInput` _returnvalue))

(event `InputAction|Interact`
  (params (Key :type "Key Structure"))
  (bind _returnvalue (`GameplayStatics.GetPlayerController` 0))
  (:`Pressed`
    (`self.DisableInput` _returnvalue)
    (`self.EnableInput` (`self.Player`) _returnvalue)
    (`Widget.RemoveFromParent` (`self.InspectionWidget`))
    (set `self.InspectionWidget` null)))

(fn `Interact`
  (params (Player :type "/Game/Programming/Core/BPC_Player Object Reference"))
  (returns (DidInteract :type Boolean))
  (return false))

(fn `UserConstructionScript`)