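; Movable pillar puzzle element that toggles between two states when its BPACOutput component fires, either once or repeatedly.
; After a delay, a timeline scaled to the animation time plays or reverses, driving any attached BPAC_Animation components.
; Triggering can also toggle interactables on attached actors and fire the smart camera if it has a fixed camera.
; The construction script can raise the cylinder to preview elevation in the editor.
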(event `self.ReceiveBeginPlay`
  (bind _bpac_output (`self.BPAC_Output`))
  ;[1 1 1] Initialisation - Bind
  (set `/Game/Programming/Core/GPE/MovableAssets/BPAC_Output.Action Repetable` (`self.Repetable`) _bpac_output)
  (set `/Game/Programming/Core/GPE/MovableAssets/BPAC_Output.Push Function` (`self.Push Function`) _bpac_output)
  (add `/Game/Programming/Core/GPE/MovableAssets/BPAC_Output.OnOutput` (`self.BPAC_Output`) (delegate `PillarMovement`))
  ;[1 1 1] Initialization of the timeline
  (`TimelineComponent.SetPlayRate` (`self.Timeline_0`) (/ 1.0 (`self.Time Animation`)))
  ;[1 1 1] Initialization for animation
  (for _array_element (`self.K2_GetComponentsByClass` "/Game/Programming/Core/GPE/MovableAssets/BPAC_Animation.BPAC_Animation_C")
    (bind _asbpac_animation (cast `/Game/Programming/Core/GPE/MovableAssets/BPAC_Animation` _array_element))
    (set `/Game/Programming/Core/GPE/MovableAssets/BPAC_Animation.Element` self _asbpac_animation)
    (`/Game/Programming/Core/GPE/MovableAssets/BPAC_Animation.Initialization` _asbpac_animation)))

(event `PillarMovement`
  ;[1 1 1] PillarMovement
  ;;[1 1 1] Desactive interact component
  (if (not (not (`self.Enable Interaction after animation`)))
    (for _array_element (`self.GetAttachedActors` true)
      (`ActorComponent.SetActive` (`self.GetComponentByClass` _array_element "/Game/Programming/Core/GPE/Items/BPAC_Interactable.BPAC_Interactable_C") (not (`self.On/Off`)) false)))
  (`self.TogglePillar` (`self.On/Off`))
  (if (not (`self.Repetable`))
    (remove `/Game/Programming/Core/GPE/MovableAssets/BPAC_Output.OnOutput` (`self.BPAC_Output`) (delegate `PillarMovement`))))

(event `TogglePillar`
  (params (Condition :type Boolean))
  (bind _returnvalue (`self.GetComponentByClass` "/Game/Programming/Core/DynamicCamera/BPAC_SmartCameraComponent.BPAC_SmartCameraComponent_C"))
  ;[1 1 1] Smooth Toggle
  (`|ExecutionSequence`
    (:`then_0`
      (`KismetSystemLibrary.Delay` (`self.Delay Before Animation`))
      (if Condition
        (bind (_direction _newtrack_0) (`Timeline|Timeline_0` :!label _label)
          (:`Update`
            ;;[1 1 1] Animations
            (for _array_element (`self.K2_GetComponentsByClass` "/Game/Programming/Core/GPE/MovableAssets/BPAC_Animation.BPAC_Animation_C")
              (bind _asbpac_animation (cast `/Game/Programming/Core/GPE/MovableAssets/BPAC_Animation` _array_element))
              (`/Game/Programming/Core/GPE/MovableAssets/BPAC_Animation.Do Animation` _asbpac_animation _newtrack_0)))
          (:`Finished`
            (set `self.On/Off` (not Condition))))
        (else
          (goto _label :!via `Reverse`))))
    (:`then_1`
      ;;[1 1 1] Camera
      (`/Engine/EditorBlueprintResources/StandardMacros.IsValid` _returnvalue
        (:`Is Valid`
          (`/Engine/EditorBlueprintResources/StandardMacros.IsValid` (`/Game/Programming/Core/DynamicCamera/BPAC_SmartCameraComponent.Fixed Camera` _returnvalue)
            (:`Is Valid`
              (`/Game/Programming/Core/DynamicCamera/BPAC_SmartCameraComponent.ExternalTrigger` _returnvalue))))))))

(fn `UserConstructionScript`
  (bind _cylinder (`self.Cylinder`))
  ;[1 1 1] See the elevation in the editor
  (if (`self.Elevated`)
    (`SceneComponent.K2_SetRelativeLocation` _cylinder (+ (`SceneComponent.RelativeLocation` _cylinder) (`KismetMathLibrary.MakeVector` 0.0 0.0 (`self.Height Elevation`))) false false)))