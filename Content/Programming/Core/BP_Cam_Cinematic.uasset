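; BP_Cam_Cinematic is a cinematic camera Blueprint that moves the player's view to a cine camera.
; StartCameraTransition disables move and look input, then cubic-blends the view to the first camera in CineCamerasArray.
; After a delay it only prints a debug value.
; The logic that blends back to the player character and restores input is disconnected, so this Blueprint leaves input ignored.
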(event `StartCameraTransition`
  (bind _returnvalue (`GameplayStatics.GetPlayerController` 0))
  (`Controller.SetIgnoreMoveInput` _returnvalue true)
  (`Controller.SetIgnoreLookInput` _returnvalue true)
  (`PlayerController.SetViewTargetWithBlend` (`GameplayStatics.GetPlayerController` 0) (`|GetArrayItem` (`self.CineCamerasArray`)) 0.6 "VTBlend_Cubic" 0.0 false)
  (`KismetSystemLibrary.Delay` 5.0)
  (`KismetSystemLibrary.PrintString` (`KismetStringLibrary.Conv_IntToString` 0)))

(event `self.ReceiveBeginPlay`)

(fn `UserConstructionScript`)