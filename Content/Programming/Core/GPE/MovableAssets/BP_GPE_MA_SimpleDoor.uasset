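; BP_GPE_MA_SimpleDoor is a door that removes itself piece by piece when its interactable component fires OnInteract.
; A Sequence starts four timelines with staggered delays, so the effect cascades across the four static meshes.
; Each timeline drives its mesh's Emissive material scalar and destroys that mesh component on finish, while the actor itself remains.
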(event `self.BPAC_Interactable.On Interact`
  (params (Player :type "/Game/Programming/Core/BPC_Player Object Reference"))
  (bind _staticmesh1 (`self.StaticMesh1`))
  (bind _staticmesh2 (`self.StaticMesh2`))
  (bind _staticmesh3 (`self.StaticMesh3`))
  (bind _staticmesh (`self.StaticMesh`))
  ;[1 1 1] Animation
  (`|ExecutionSequence`
    (:`then_0`
      (bind (_direction _value) (`Timeline|IntoDeath`)
        (:`Update`
          (`MeshComponent.SetScalarParameterValueOnMaterials` _staticmesh "Emissive" _value))
        (:`Finished`
          (`ActorComponent.K2_DestroyComponent` _staticmesh))))
    (:`then_1`
      (`KismetSystemLibrary.Delay` 0.4)
      (bind (_direction_2 _value_2) (`Timeline|Timeline_0`)
        (:`Update`
          (`MeshComponent.SetScalarParameterValueOnMaterials` _staticmesh1 "Emissive" _value_2))
        (:`Finished`
          (`ActorComponent.K2_DestroyComponent` _staticmesh1))))
    (:`then_2`
      (`KismetSystemLibrary.Delay` 0.9)
      (bind (_direction_3 _value_3) (`Timeline|Timeline_1`)
        (:`Update`
          (`MeshComponent.SetScalarParameterValueOnMaterials` _staticmesh2 "Emissive" _value_3))
        (:`Finished`
          (`ActorComponent.K2_DestroyComponent` _staticmesh2))))
    (:`then_3`
      (`KismetSystemLibrary.Delay` 1.3)
      (bind (_direction_4 _value_4) (`Timeline|Timeline_2`)
        (:`Update`
          (`MeshComponent.SetScalarParameterValueOnMaterials` _staticmesh3 "Emissive" _value_4))
        (:`Finished`
          (`ActorComponent.K2_DestroyComponent` _staticmesh3))))))

(fn `UserConstructionScript`)