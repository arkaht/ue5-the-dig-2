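; Movable statue puzzle element that the player toggles between two states, updating its BPAC_Input component.
; An optional BPAC_Output keeps interaction disabled until it fires.
; Each toggle waits a delay, then plays one timeline forward or in reverse to drive all BPAC_Animation components, blocking interaction meanwhile and re-offering it to the player afterward.
; The state saves through BPSG_Output, and loading snaps the animation components into position without replaying.
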(event `self.ReceiveBeginPlay`
  (bind _returnvalue (`self.GetComponentByClass` "/Game/Programming/Core/GPE/MovableAssets/BPAC_Output.BPAC_Output_C"))
  ;[1 1 1] Initialization
  (`/Game/Programming/Core/GPE/MovableAssets/BPAC_Input.Set_Active` (`self.GetComponentByClass` "/Game/Programming/Core/GPE/MovableAssets/BPAC_Input.BPAC_Input_C") (`self.On/Off`))
  ;;[1 1 1] If Ouput exist
  (`/Engine/EditorBlueprintResources/StandardMacros.IsValid` _returnvalue
    (:`Is Valid`
      (`ActorComponent.SetActive` (`self.BPAC_Interactable`) false false)
      (add `/Game/Programming/Core/GPE/MovableAssets/BPAC_Output.OnOutput` _returnvalue (delegate `Activation`)))
    (:`Is Not Valid`
      _))
  ;;[1 1 1] Initialization of the timeline
  (`TimelineComponent.SetPlayRate` (`self.Timeline_0`) (/ 1.0 (`self.Time Animation`)))
  ;;[1 1 1] Initialization for animation
  (for _array_element (`self.K2_GetComponentsByClass` "/Game/Programming/Core/GPE/MovableAssets/BPAC_Animation.BPAC_Animation_C")
    (bind _asbpac_animation (cast `/Game/Programming/Core/GPE/MovableAssets/BPAC_Animation` _array_element))
    (set `/Game/Programming/Core/GPE/MovableAssets/BPAC_Animation.Element` self _asbpac_animation)
    (`/Game/Programming/Core/GPE/MovableAssets/BPAC_Animation.Initialization` _asbpac_animation)))

(event `Activation`
  ;[1 1 1] If Ouput exist
  ;;[1 1 1] If Ouput call
  (`ActorComponent.SetActive` (`self.BPAC_Interactable`) true false))

(event `self.BPAC_Interactable.On Interact`
  (params (Player :type "/Game/Programming/Core/BPC_Player Object Reference"))
  ;[1 1 1] Interaction
  (`self.PillarMovement`))

(event `PillarMovement`
  ;[1 1 1] PillarMovement
  (`self.TogglePillar` (`self.On/Off`)))

(event `TogglePillar`
  (params (Condition :type Boolean))
  (bind _returnvalue (`self.GetComponentByClass` "/Game/Programming/Core/GPE/MovableAssets/BPAC_Input.BPAC_Input_C"))
  ;[1 1 1] Smooth Toggle
  (set `self.On/Off` (not Condition))
  (set `self.Is In Animation` true)
  ;;[0 1 0.01469 0.33] Status modify
  (`/Engine/EditorBlueprintResources/StandardMacros.IsValid` _returnvalue
    (:`Is Valid`
      (`/Game/Programming/Core/GPE/MovableAssets/BPAC_Input.Set_Active` _returnvalue (`self.On/Off`)))
    (:`Is Not Valid`
      _))
  (`KismetSystemLibrary.Delay` (`self.Delay Before Animation`))
  (if (`self.On/Off Reverse`)
    (bind (_direction _newtrack_0) (`Timeline|Timeline_0` :!via `PlayFromStart` :!label _label)
      (:`Update`
        ;;[1 1 1] Animations
        (for _array_element (`self.K2_GetComponentsByClass` "/Game/Programming/Core/GPE/MovableAssets/BPAC_Animation.BPAC_Animation_C")
          (bind _asbpac_animation (cast `/Game/Programming/Core/GPE/MovableAssets/BPAC_Animation` _array_element))
          (`/Game/Programming/Core/GPE/MovableAssets/BPAC_Animation.Do Animation` _asbpac_animation _newtrack_0)))
      (:`Finished`
        (set `self.On/Off Reverse` (not (`self.On/Off Reverse`)))
        (set `self.Is In Animation` false)
        ;;[1 1 1 0.33] Try re-Giving Interaction
        (bind _asbpc_player (cast `/Game/Programming/Core/BPC_Player` (`GameplayStatics.GetPlayerCharacter` 0)))
        (`/Game/Programming/Core/BPC_Player.Try Set Current Interactable` _asbpc_player (`self.BPAC_Interactable`) true true)))
    (else
      (goto _label :!via `ReverseFromEnd`))))

(event `/Game/Programming/Core/Savers/BPI_Saveable.Load Data`
  (params (Data :type "SaveGame Object Reference"))
  ;[1 1 1 0.33] Load Save
  (bind _asbpsg_output (cast `/Game/Programming/Core/Savers/Data/BPSG_Output` Data))
  (bind _is_active (`/Game/Programming/Core/Savers/Data/BPSG_Output.Is Active` _asbpsg_output))
  ;;[1 1 1 0.33] Set Active on Change
  (if (!= _is_active (`self.On/Off`))
    (bind _output_get (set `self.On/Off` _is_active))
    ;;[1 1 1 0.33] Repositioning
    (set `self.On/Off Reverse` (not _output_get))
    (for _array_element (`self.K2_GetComponentsByClass` "/Game/Programming/Core/GPE/MovableAssets/BPAC_Animation.BPAC_Animation_C")
      (bind _asbpac_animation (cast `/Game/Programming/Core/GPE/MovableAssets/BPAC_Animation` _array_element))
      (`/Game/Programming/Core/GPE/MovableAssets/BPAC_Animation.Repositioning` _asbpac_animation (`self.On/Off Reverse`)))
    (set `/Game/Programming/Core/GPE/MovableAssets/BPAC_Input.Is Active` (`self.On/Off`) (`self.GetComponentByClass` "/Game/Programming/Core/GPE/MovableAssets/BPAC_Input.BPAC_Input_C"))))

(fn `Can Interact`
  (params (Player :type "/Game/Programming/Core/BPC_Player Object Reference"))
  (returns (`Can Interact` :type Boolean))
  (return (not (`self.Is In Animation`))))

(fn `Get Save Data`
  (returns (Data :type "SaveGame Object Reference"))
  (bind _returnvalue (`GameplayStatics.CreateSaveGameObject` "/Game/Programming/Core/Savers/Data/BPSG_Output.BPSG_Output_C"))
  (set `/Game/Programming/Core/Savers/Data/BPSG_Output.Is Active` (`self.On/Off`) _returnvalue)
  (return _returnvalue))

(fn `UserConstructionScript`)