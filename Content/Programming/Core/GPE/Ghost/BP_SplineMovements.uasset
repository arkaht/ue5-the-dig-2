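; Ghost set piece that spawns an idle ghost FX at its start location, then flies a ghost actor along a spline when the player enters the trigger box.
; The first overlap plays a timeline scaled by TimelineLenght that sets the actor's location and tangent-facing rotation, then destroys it after a delay.
; Meanwhile, the idle FX has its Niagara spawn rates zeroed and is destroyed two seconds later.
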(event `self.ReceiveBeginPlay`
  ;[0 0.5689 1] Spawn the Ghost at the launch of the game
  (bind _returnvalue (`|SpawnActorFromClass` "/Game/Art/4_FX/Actors/BPC_SpawnGhostFX.BPC_SpawnGhostFX_C" (`KismetMathLibrary.MakeTransform` (`self.Ghost Start location`)) "Undefined" "OverrideRootScale" null null))
  (set `self.FX UpDown Ghost` _returnvalue))

(event `self.Box.OnComponentBeginOverlap`
  (params (OverlappedComponent :type "PrimitiveComponent Object Reference") (OtherActor :type "Actor Object Reference") (OtherComp :type "PrimitiveComponent Object Reference") (OtherBodyIndex :type Integer) (bFromSweep :type Boolean) (SweepResult :type "HitResult Structure (by ref)"))
  ;[0.1224 1 0] Trigger the movements of the ghost along the spline + destroy the first ghost
  (`/Engine/EditorBlueprintResources/StandardMacros.DoOnce` false
    (:`Completed`
      (cast `/Game/Programming/Core/BPC_Player` OtherActor)
      (set `self.Is Seeing Player` true)
      (if (`self.Is Seeing Player`)
        (`TimelineComponent.SetPlayRate` (`self.GhostMovements`) (/ 1.0 (`self.Timeline Lenght`)))
        (`self.Play Timeline`)
        (`self.End UpDown Ghost Particles`)
        (`KismetSystemLibrary.Delay` 2.0)
        (`self.K2_DestroyActor` (`self.FX UpDown Ghost`))))))

(event `Play Timeline`
  (bind _spline (`self.Spline`))
  (bind _spline_2 (`self.Spline`))
  (bind _actor (`self.Actor`))
  ;[1 0.9797 0] Timeline + movements along the spline
  (bind (_direction _movements) (`Timeline|GhostMovements` :!via `PlayFromStart`)
    (:`Update`
      (bind _returnvalue (`KismetMathLibrary.Lerp` 0.0 (`SplineComponent.GetDistanceAlongSplineAtSplinePoint` _spline (- (`SplineComponent.GetNumberOfSplinePoints` _spline) 1)) _movements))
      (`self.K2_SetActorLocation` _actor (`SplineComponent.GetLocationAtDistanceAlongSpline` _spline_2 _returnvalue "World") false false)
      (`self.K2_SetActorRotation` _actor (`KismetMathLibrary.Conv_VectorToRotator` (`SplineComponent.GetTangentAtDistanceAlongSpline` _spline_2 _returnvalue "World")) false)
      (`KismetSystemLibrary.Delay` (`self.Delay Before Destruction`))
      (`self.K2_DestroyActor` (`self.Actor`)))))

(fn `End Ghost Particles`
  (bind _fx_ghost (`self.FX Ghost`))
  (bind _ghosttofollow (`/Game/Programming/Core/GPE/Ghost/BP_GhostFollow.GhostToFollow` _fx_ghost))
  (`/Engine/EditorBlueprintResources/StandardMacros.IsValid` _fx_ghost
    (:`Is Valid`
      (`|ExecutionSequence`
        (:`then_0`
          (`NiagaraComponent.SetVariableFloat` _ghosttofollow "SpawnRate_Vortex" 0.0))
        (:`then_1`
          (`NiagaraComponent.SetVariableFloat` _ghosttofollow "SpawnRate_Vortex2" 0.0))
        (:`then_2`
          (`NiagaraComponent.SetVariableFloat` _ghosttofollow "SpawnRate_GhostParticles" 0.0))))))

(fn `End UpDown Ghost Particles`
  (bind _fx_updown_ghost (`self.FX UpDown Ghost`))
  (bind _fx_ghost (`/Game/Art/4_FX/Actors/BPC_SpawnGhostFX.FX_Ghost` _fx_updown_ghost))
  (`/Engine/EditorBlueprintResources/StandardMacros.IsValid` _fx_updown_ghost
    (:`Is Valid`
      (`|ExecutionSequence`
        (:`then_0`
          (`NiagaraComponent.SetVariableFloat` _fx_ghost "SpawnRate_Vortex" 0.0))
        (:`then_1`
          (`NiagaraComponent.SetVariableFloat` _fx_ghost "SpawnRate_Vortex2" 0.0))
        (:`then_2`
          (`NiagaraComponent.SetVariableFloat` _fx_ghost "SpawnRate_GhostParticles" 0.0))))))

(fn `UserConstructionScript`
  (`self.K2_SetActorLocation` (`self.Actor`) (`SplineComponent.GetLocationAtSplinePoint` (`self.Spline`) 0 "Local") false false))