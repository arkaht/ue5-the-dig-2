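; BP_GhostToFollow is a ghost character that leads the way to a preset destination once it spots a character.
; It sets its walk speed on BeginPlay, then pawn sensing triggers an AI move to GhostDestination.
; On arrival, it zeroes the spawn rates of its Niagara vortex and ghost particle emitters so the effect fades out.
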(event `self.ReceiveBeginPlay`
  (set `CharacterMovementComponent.MaxWalkSpeed` (`self.Speed`) (`self.CharacterMovement`)))

(event `self.PawnSensing.OnSeePawn`
  (params (Pawn :type "Pawn Object Reference"))
  (bind _ghosttofollow (`self.GhostToFollow`))
  (cast `Character` Pawn)
  (`|AIMoveTo` self (`self.Ghost Destination`) null 2.5
    (:`OnSuccess`
      (`|ExecutionSequence`
        (:`then_0`
          (`NiagaraComponent.SetVariableFloat` _ghosttofollow "User.SpawnRate_Vortex" 0.0))
        (:`then_1`
          (`NiagaraComponent.SetVariableFloat` _ghosttofollow "User.SpawnRate_Vortex2" 0.0))
        (:`then_2`
          (`NiagaraComponent.SetVariableFloat` _ghosttofollow "User.SpawnRate_GhostParticles" 0.0))))))

(fn `UserConstructionScript`)